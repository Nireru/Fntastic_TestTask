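; Turtle character that walks to BPC_ArrivingPoint_2 in a stop-and-go rhythm, using inherited start-sound and end functions.
; BeginPlay starts AI MoveTo alongside a delay loop that periodically disables movement, pausing sound and particles, then restores NavWalking.
; A proximity check stops the loop directly.
; Move success or failure clears the Moving flag, so a subsequent loop check calls FuncEndOperations.
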(event EventBeginPlay
  (|CallParentFunction)
  ;[1 1 1] Getting ArrivingPoint_2 location
  (bind _returnvalue (Actor|GetActorOfClass "/Game/Others/ArrivingPoint/BPC_ArrivingPoint_2.BPC_ArrivingPoint_2_C"))
  (bind _asbpc_arriving_point_2 (Utilities|Casting|CastToBPC_ArrivingPoint_2 _returnvalue)
    (:then
      (bind _output_get (Variables|Default|SetArrivingPoint_2%20Location (Transformation|GetWorldLocation (Variables|/Game/Others/ArrivingPoint/BP_ArrivingPoint.BP_ArrivingPoint_C|GetArriving%20Point _asbpc_arriving_point_2))))
      ;[1 1 1] Going to Arriving Point (for 1 sec)
      (AI|AIMoveTo self _output_get 0 5.0 false
        (:then
          (CallFunction|FuncStartSound)
          ;[1 1 1] Loop start
          (Variables|Default|SetMoving? true)
          (if (Variables|Default|GetMoving?) :!label _label
            (Utilities|FlowControl|Delay 1.0) ; Moving time delay
            ;[1 1 1] Stop turtle for 0.5 sec, pause sound and disable particles
            (Pawn|Components|CharacterMovement|DisableMovement (Variables|Character|GetCharacterMovement))
            (Components|Activation|Deactivate (Variables|Default|GetParticle))
            (Class|AudioComponent|SetPaused (Variables|Default|Get2DSound) true)
            (Utilities|FlowControl|Delay 0.5)
            ;[1 1 1] Turtle moves again, particle activates, sound unpauses
            (Pawn|Components|CharacterMovement|SetMovementMode (Variables|Character|GetCharacterMovement) "MOVE_NavWalking" 0)
            (Components|Activation|Activate (Variables|Default|GetParticle) false)
            (Class|AudioComponent|SetPaused (Variables|Default|Get2DSound) false)
            (Utilities|NearArrivingPoint?
              (:True
                (Variables|Default|SetMoving? false))
              (:False
                (goto _label)))
            (else
              (CallFunction|FuncEndOperations))))
        (:OnSuccess
          (Variables|Default|SetMoving? false))
        (:OnFail
          (Variables|Default|SetMoving? false))))
    (:CastFailed
      (Development|PrintString "Cast Failed"))))

(fn ConstructionScript
  (|CallParentFunction))