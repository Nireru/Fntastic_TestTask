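; Third turtle variant: an AI pawn that tries to travel to the player controller's third destination, using Nest 3 as its fallback point.
; A gated loop re-issues AI MoveTo toward the destination and back to the nest on short delays, without waiting for moves to finish.
; Arrival closes the gate, runs success effects and destroys the turtle.
; A parallel timeout triggers failure handling, unpossesses and destroys it if it hasn't arrived.
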(event EventBeginPlay
  (|CallParentFunction)
  ;[1 1 1] Getting locations of objects in level
  (bind _asbp_player_controller (Utilities|Casting|CastToBP_PlayerController (Game|GetPlayerController 0))
    (:then
      (Variables|Default|SetArrivingPoint_3%20Location (Variables|/Game/Others/BP_PlayerController.BP_PlayerController_C|GetThirdDestination _asbp_player_controller))
      (bind _returnvalue (Actor|GetActorOfClass "/Game/Nest/BPC_Nest_3.BPC_Nest_3_C"))
      (Variables|Default|SetNestPoint_3%20Location (Transformation|GetWorldLocation (Variables|/Game/Nest/Material/BP_Nest.BP_Nest_C|GetNest _returnvalue)))
      (CallFunction|FuncStartingSoundPlay)
      (Utilities|FlowControl|Sequence
        (:then_0
          (Utilities|FlowControl|Gate false :!label _label
            (:Exit
              (Utilities|ForwardandBackwardSequence
                (:Fail
                  (goto _label))
                (:Success
                  (Utilities|FlowControl|Sequence
                    (:then_0
                      (goto _label Close))
                    (:then_1
                      (bind _particle_ref (CallFunction|FuncSucceedArriving))
                      (Utilities|FlowControl|Delay 2.0)
                      (Components|DestroyComponent _particle_ref) ; Destroying "win" spawned particle
                      (Utilities|FlowControl|Delay 3.0)
                      (Actor|DestroyActor))))))))
        (:then_1
          ;[1 1 1] Because "AI Move To" always "fails" i made 15 sec. limit
          (Utilities|FlowControl|Delay 15.0)
          (if (not (Variables|Default|GetArrived?)) ; If true, then he anyway will be deleted by another node
            (Development|PrintString "Turtle didn't arrive in 15 sec. He will be doomed in 3 sec." true true "(R=1.000000,G=0.000000,B=0.031044,A=1.000000)")
            (Utilities|FlowControl|Sequence
              (:then_0
                (goto _label Close))
              (:then_1
                (CallFunction|FuncFailArriving)
                (Pawn|UnPossess (Pawn|GetController))
                (Utilities|FlowControl|Delay 3.0)
                (Actor|DestroyActor)))))))
    (:CastFailed
      (Development|PrintString "BP_PlayerController Cast Failed (Third Turtle)"))))

(fn ConstructionScript
  (|CallParentFunction))