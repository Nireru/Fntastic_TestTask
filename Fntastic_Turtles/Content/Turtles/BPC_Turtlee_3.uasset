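; Turtle pawn Blueprint, variant 3, that makes back-and-forth progress from its nest toward its arriving point.
; On BeginPlay it caches both level actors' locations, starts a sound and enters a movement loop.
; AI MoveTo's immediate exec drives timed switching: one second toward the arriving point, half a second back toward the nest.
; Reaching the arriving point clears the Moving flag and calls the end-operations function, stopping the loop.
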(event EventBeginPlay
  (|CallParentFunction)
  ;[1 1 1] Getting locations of objects in level
  (bind _returnvalue (Actor|GetActorOfClass "/Game/Others/ArrivingPoint/BPC_ArrivingPoint_3.BPC_ArrivingPoint_3_C"))
  (bind _asbpc_arriving_point_3 (Utilities|Casting|CastToBPC_ArrivingPoint_3 _returnvalue)
    (:then
      (Variables|Default|SetArrivingPoint_3%20Location (Transformation|GetWorldLocation (Variables|/Game/Others/ArrivingPoint/BP_ArrivingPoint.BP_ArrivingPoint_C|GetArriving%20Point _asbpc_arriving_point_3)))
      (bind _returnvalue_2 (Actor|GetActorOfClass "/Game/Nest/BPC_Nest_3.BPC_Nest_3_C"))
      (bind _asbpc_nest_3 (Utilities|Casting|CastToBPC_Nest_3 _returnvalue_2)
        (:then
          (Variables|Default|SetNestPoint_3%20Location (Transformation|GetWorldLocation (Variables|/Game/Nest/BP_Nest.BP_Nest_C|GetNest _asbpc_nest_3)))
          (CallFunction|FuncStartSound)
          ;[1 1 1] Start of the loop
          (Variables|Default|SetMoving? true)
          (if (Variables|Default|GetMoving?) :!label _label
            ;[1 1 1] Move to BPC_ArrivingPoint_3 for 1 sec. If succed/fail set "Moving?" to 0
            (AI|AIMoveTo self (Variables|Default|GetArrivingPoint_3%20Location) 0 5.0 false
              (:then
                (Utilities|FlowControl|Delay 1.0))
              (:OnSuccess
                ;[1 1 1] Parrent "Func End Operations" here because "AIMoveTo" plays WITH standart "out" exec that triggers "false" loop route second time
                (Variables|Default|SetMoving? false)
                (CallFunction|FuncEndOperations)))
            ;[1 1 1] If moving set to 0 then skip next step and go to beggining of the loop to end it. Otherwise continue sequence
            (if (Variables|Default|GetMoving?)
              ;[1 1 1] Move to BPC_Nest_3 for 0.5 sec. Then go to begging of the loop
              (AI|AIMoveTo self (Variables|Default|GetNestPoint_3%20Location) 0 5.0 true
                (:then
                  (Utilities|FlowControl|Delay 0.5)
                  (goto _label)))
              (else
                (goto _label)))))
        (:CastFailed
          (Development|PrintString "BPC_Nest_3 Cast Failed"))))
    (:CastFailed
      (Development|PrintString "BPC_ArrivingPoint_3 Cast Failed"))))

(fn ConstructionScript
  (|CallParentFunction))