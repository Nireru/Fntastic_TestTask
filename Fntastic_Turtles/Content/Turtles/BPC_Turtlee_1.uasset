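; BPC_Turtlee_1 is a turtle pawn Blueprint that travels to its arrival point when play begins.
; BeginPlay finds the BPC_ArrivingPoint_1 actor, calls FuncStartSound, then uses AI Move To toward that actor's ArrivingPoint component location.
; A successful move calls FuncEndOperations, while a failed cast prints an error message.
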(event EventBeginPlay
  (|CallParentFunction)
  ;[1 1 1] Getting AriivingPoint_1 location
  (bind _returnvalue (Actor|GetActorOfClass "/Game/Others/ArrivingPoint/BPC_ArrivingPoint_1.BPC_ArrivingPoint_1_C"))
  (bind _asbpc_arriving_point_1 (Utilities|Casting|CastToBPC_ArrivingPoint_1 _returnvalue)
    (:then
      (CallFunction|FuncStartSound)
      ;[1 1 1] Moving to location
      (AI|AIMoveTo self (Transformation|GetWorldLocation (Variables|/Game/Others/ArrivingPoint/BP_ArrivingPoint.BP_ArrivingPoint_C|GetArriving%20Point _asbpc_arriving_point_1)) 0 5.0 false
        (:OnSuccess
          (CallFunction|FuncEndOperations))))
    (:CastFailed
      (Development|PrintString "BPC_Turtle_1 Cast Failed"))))

(fn ConstructionScript
  (|CallParentFunction))