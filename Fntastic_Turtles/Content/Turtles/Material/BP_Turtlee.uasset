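; BP_Turtlee is a turtle Blueprint whose functions handle audio and particle feedback for starting, reaching or failing to reach a destination.
; The start function spawns a 2D music track and stores its component.
; Success and failure both destroy the existing walking particle and stop the stored sound, with validity checks.
; Success then plays a crowd sound and spawns a finish emitter at the turtle's location.
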(fn ConstructionScript)

(fn FuncSucceedArriving
  (bind _returnvalue (Transformation|GetActorLocation))
  (bind _2dsound (Variables|Default|Get2DSound))
  (bind _particle (Variables|Default|GetParticle))
  ;[1 1 1] Stop "walking" particle and sound
  (Utilities|IsValid _particle
    (:Is%20Valid
      (Components|DestroyComponent _particle)
      (Utilities|IsValid _2dsound
        (:Is%20Valid
          (Audio|Components|Audio|Stop _2dsound)
          ;[1 1 1] Start "finish" particle and sound
          (Audio|PlaySoundatLocation "/Game/Others/Sounds/human-crowd-138-sound-effect-3976441.human-crowd-138-sound-effect-3976441" _returnvalue "0, 0, 0" 1.0 1.0 0.0 0 0 0)
          (bind _returnvalue_2 (Effects|SpawnEmitteratLocation "/Game/Others/Particles/PS_TurtleFinish.PS_TurtleFinish" _returnvalue)))
        (:Is%20Not%20Valid
          _)))
    (:Is%20Not%20Valid
      _))
  (return _returnvalue_2))

(fn FuncStartingSoundPlay
  (bind _returnvalue (Audio|SpawnSound2D "/Game/Others/Sounds/alex-productions-epic-cinematic-trailer-elite.alex-productions-epic-cinematic-trailer-elite" 1.0 1.0 0.0 0))
  (Variables|Default|Set2DSound _returnvalue))

(fn FuncFailArriving
  (bind _2dsound (Variables|Default|Get2DSound))
  (bind _particle (Variables|Default|GetParticle))
  ;[1 1 1] Stop "walking" particle and sound
  (Utilities|IsValid _particle
    (:Is%20Valid
      (Components|DestroyComponent _particle)
      (Utilities|IsValid _2dsound
        (:Is%20Valid
          (Audio|Components|Audio|Stop _2dsound))
        (:Is%20Not%20Valid
          _)))
    (:Is%20Not%20Valid
      _))
  (return))