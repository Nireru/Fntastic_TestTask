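; Second turtle character, a child Blueprint that AI-moves to the player controller's SecondDestination in a stop-and-go rhythm.
; A looping Gate drives the PauseContinueSequence macro, which alternately disables and restores walking, along with the particle and 2D sound.
; Arrival or failure calls the matching outcome function, then closes the Gate and destroys the actor after a delay, with the win particle removed first on success.
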(event EventBeginPlay
  (|CallParentFunction)
  ;[1 1 1] Getting TargetPoint2 location
  (bind _asbp_player_controller (Utilities|Casting|CastToBP_PlayerController (Game|GetPlayerController 0))
    (:then
      (AI|AIMoveTo self (Variables|/Game/Others/BP_PlayerController.BP_PlayerController_C|GetSecondDestination _asbp_player_controller) 0 5.0 false
        (:then
          (CallFunction|FuncStartingSoundPlay)
          (Utilities|FlowControl|Gate false :!label _label
            (:Exit
              (Utilities|PauseContinueSequence ; Go for 1 sec, stop for 0,5 sec
                (:Out
                  (goto _label))))))
        (:OnSuccess
          (Development|PrintString "Second  Turtle Success")
          (bind _particle_ref (CallFunction|FuncSucceedArriving))
          (Utilities|FlowControl|Delay 2.0)
          (Components|DestroyComponent _particle_ref) ; Destroying "win" spawned particle
        )
        (:OnFail
          (Development|PrintString "Second Turtle Fail")
          (CallFunction|FuncFailArriving)))
      (Utilities|FlowControl|Sequence
        (:then_0
          (goto _label Close))
        (:then_1
          (Utilities|FlowControl|Delay 3.0)
          (Actor|DestroyActor))))
    (:CastFailed
      (Development|PrintString "Cast Failed"))))

(fn ConstructionScript
  (|CallParentFunction))

(fn FuncPauseMovement
  (bind _2dsound (Variables|Default|Get2DSound))
  (bind _charactermovement (Variables|Character|GetCharacterMovement))
  (bind _particle (Variables|Default|GetParticle))
  (Utilities|IsValid _charactermovement
    (:Is%20Valid
      (Pawn|Components|CharacterMovement|DisableMovement _charactermovement)
      (Utilities|IsValid _particle
        (:Is%20Valid
          (Components|Activation|Deactivate _particle)
          (Utilities|IsValid _2dsound
            (:Is%20Valid
              (Class|AudioComponent|SetPaused _2dsound true))
            (:Is%20Not%20Valid
              _)))
        (:Is%20Not%20Valid
          _)))
    (:Is%20Not%20Valid
      _))
  (return))

(fn FuncContinueMovement
  (bind _particle (Variables|Default|GetParticle))
  (bind _charactermovement (Variables|Character|GetCharacterMovement))
  (bind _2dsound (Variables|Default|Get2DSound))
  (Utilities|IsValid _charactermovement
    (:Is%20Valid
      (Pawn|Components|CharacterMovement|SetMovementMode _charactermovement "MOVE_Walking" 0)
      (Utilities|IsValid _particle
        (:Is%20Valid
          (Components|Activation|Activate _particle false)
          (Utilities|IsValid _2dsound
            (:Is%20Valid
              (Class|AudioComponent|SetPaused _2dsound false))
            (:Is%20Not%20Valid
              _)))
        (:Is%20Not%20Valid
          _)))
    (:Is%20Not%20Valid
      _))
  (return))