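; Turtle actor Blueprint with helper functions for the audio and particle feedback at the start and end of its run.
; Func_StartSound spawns a 2D cinematic track and keeps a reference to it.
; Func_EndOperations deactivates the fire particle, spawns a finish emitter at the turtle's location, stops the stored track and plays a crowd sound there as the win cue.
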(fn ConstructionScript)

(fn FuncEndOperations
  ;[1 1 1] Stopping fire particle
  (Components|Activation|Deactivate (Variables|Default|GetParticle))
  ;[1 1 1] Starting finish particle
  (Effects|SpawnEmitteratLocation "/Game/Others/Particles/PS_TurtleFinish.PS_TurtleFinish" (Transformation|GetActorLocation))
  ;[1 1 1] Stop "walking sound" start "win" song
  (Audio|Components|Audio|Stop (Variables|Default|Get2DSound))
  (Audio|PlaySoundatLocation "/Game/Others/Sounds/human-crowd-138-sound-effect-3976441.human-crowd-138-sound-effect-3976441" (Transformation|GetActorLocation) "0, 0, 0" 1.0 1.0 0.0 0 0 0))

(fn FuncStartSound
  (bind _returnvalue (Audio|SpawnSound2D "/Game/Others/Sounds/alex-productions-epic-cinematic-trailer-elite.alex-productions-epic-cinematic-trailer-elite" 1.0 1.0 0.0 0))
  (Variables|Default|Set2DSound _returnvalue))