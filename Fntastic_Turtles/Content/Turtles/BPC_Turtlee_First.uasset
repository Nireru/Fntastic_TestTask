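; Turtle pawn Blueprint for the first turtle, which walks to a destination on spawn and removes itself afterwards.
; On BeginPlay it reads FirstDestination from BP_PlayerController and runs AIMoveTo, starting walking sound and particles.
; Success plays win effects and clears that particle after a delay; failure stops the moving effects.
; Both outcomes print a debug message, then destroy the actor after a further delay.
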(event EventBeginPlay
  (|CallParentFunction)
  ;[1 1 1] Cast to get Destination info
  (bind _asbp_player_controller (Utilities|Casting|CastToBP_PlayerController (Game|GetPlayerController 0))
    (:then
      (AI|AIMoveTo self (Variables|/Game/Others/BP_PlayerController.BP_PlayerController_C|GetFirstDestination _asbp_player_controller) 0 5.0 false
        (:then
          (CallFunction|FuncStartingSoundPlay) ; Plays "walking" sound and particle
        )
        (:OnSuccess
          (bind _particle_ref (CallFunction|FuncSucceedArriving)) ; Same as Fail but also plays "win" sound and particles
          (Development|PrintString "First Turtle Succed")
          (Utilities|FlowControl|Delay 2.0)
          (Components|DestroyComponent _particle_ref) ; Destroying "win" spawned particle
          (Utilities|FlowControl|Delay 3.0 :!label _label)
          (Actor|DestroyActor))
        (:OnFail
          (CallFunction|FuncFailArriving) ; Stops sound and disables "moving" particle
          (Development|PrintString "First Turtle Failed")
          (goto _label))))
    (:CastFailed
      (Development|PrintString "BP_PlayerController Cast Failed (FirstTurtle)"))))

(fn ConstructionScript
  (|CallParentFunction))