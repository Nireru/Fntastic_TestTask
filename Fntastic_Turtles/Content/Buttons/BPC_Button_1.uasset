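; Clickable button Blueprint that spawns a BPC_Turtlee_First at a random point inside the spawn box of the level's BPC_Nest_1.
; A hitbox click passes through a DoOnce, then spawns the turtle and calls FuncSpawnSoundParticles at its location.
; After a short delay it destroys the particle component and fires OnClickedFinish, which resets the DoOnce to block click spamming during each cycle.
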(event OnClicked(Button_HitBox)
  (params (TouchedComponent :type Primitive%20Component%20Object%20Reference) (ButtonPressed :type Key%20Structure :default "None"))
  (Development|PrintString "Clicked Button 1")
  ;[0 0.3 1] NEW: Prevents constant staying of particle in the level. Also prevents button spamming
  (Utilities|FlowControl|DoOnce false
    (:Completed
      ;[1 1 1] Get location info
      (bind _returnvalue (Actor|GetActorOfClass "/Game/Nest/BPC_Nest_1.BPC_Nest_1_C"))
      ;[1 1 1] Spawn Turtle & play sound & spawn particle then destroy(particle) after 2 sec delay
      (bind _returnvalue_2 (Game|SpawnActorfromClass "/Game/Turtles/BPC_Turtlee_First.BPC_Turtlee_First_C" (Math|Conversions|ToTransform(Vector) (Math|Random|RandomPointinBoundingBox (Transformation|GetWorldLocation (Variables|/Game/Nest/Material/BP_Nest.BP_Nest_C|GetTurtle_SpawnBox _returnvalue)) (Components|Box|GetScaledBoxExtent (Variables|/Game/Nest/Material/BP_Nest.BP_Nest_C|GetTurtle_SpawnBox _returnvalue)))) "AdjustIfPossibleButDontSpawnIfColliding" 0 0))
      (bind _particle_reference (Default|FuncSpawnSound&Particles self (Transformation|GetActorLocation _returnvalue_2)))
      (Utilities|FlowControl|Delay 2.0)
      (Components|DestroyComponent _particle_reference)
      ;;[0 0.3 1] NEW: Ending event  that plays when all nodes finished their job.
      (CallFunction|OnClickedFinish))))

(event Custom|On%20Clicked%20Finish
  ;[0 0.3 1] NEW: Prevents constant staying of particle in the level. Also prevents button spamming
  (Utilities|FlowControl|DoOnce false) ; enters at Reset
)

(fn ConstructionScript
  (|CallParentFunction))