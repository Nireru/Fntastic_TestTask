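; Clickable button actor that spawns a BPC_Turtlee_3 turtle at the BPC_Nest_3 nest.
; Clicking its hitbox finds the nest by class and spawns the turtle at a random point inside the nest's TurtleSpawnBox, adjusting for collisions.
; A sound plays at the turtle's location, while a spawn particle appears at a separately randomized point in the box and is destroyed after a short delay.
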(event OnClicked(Button_HitBox)
  (params (TouchedComponent :type Primitive%20Component%20Object%20Reference) (ButtonPressed :type Key%20Structure))
  ;[1 1 1] Get location info
  (bind _returnvalue (Actor|GetActorOfClass "/Game/Nest/BPC_Nest_3.BPC_Nest_3_C"))
  (bind _asbpc_nest_3 (Utilities|Casting|CastToBPC_Nest_3 _returnvalue)
    (:then
      ;[1 1 1] Spawn Turtle & play sound & spawn particle then destroy(particle) after 2 sec
      (bind _returnvalue_2 (Game|SpawnActorfromClass "/Game/Turtles/BPC_Turtlee_3.BPC_Turtlee_3_C" (Math|Conversions|ToTransform(Vector) (Math|Random|RandomPointinBoundingBox (Transformation|GetWorldLocation (Variables|/Game/Nest/BP_Nest.BP_Nest_C|GetTurtle_SpawnBox _asbpc_nest_3)) (Components|Box|GetScaledBoxExtent (Variables|/Game/Nest/BP_Nest.BP_Nest_C|GetTurtle_SpawnBox _asbpc_nest_3)))) "AdjustIfPossibleButDontSpawnIfColliding" 0 0))
      (Audio|PlaySoundatLocation "/Game/Others/Sounds/human-crowdstudio-176-sound-effect-78527833.human-crowdstudio-176-sound-effect-78527833" (Transformation|GetActorLocation _returnvalue_2) "0, 0, 0" 1.0 1.0 0.0 0 0 0)
      (bind _returnvalue_3 (Effects|SpawnEmitteratLocation "/Game/Others/Particles/PS_TurtleSpawn.PS_TurtleSpawn" (Math|Random|RandomPointinBoundingBox (Transformation|GetWorldLocation (Variables|/Game/Nest/BP_Nest.BP_Nest_C|GetTurtle_SpawnBox _asbpc_nest_3)) (Components|Box|GetScaledBoxExtent (Variables|/Game/Nest/BP_Nest.BP_Nest_C|GetTurtle_SpawnBox _asbpc_nest_3)))))
      (Utilities|FlowControl|Delay 2.0)
      (Components|DestroyComponent _returnvalue_3))
    (:CastFailed
      (Development|PrintString "BPC_Nest_3 Cast Failed"))))

(fn ConstructionScript
  (|CallParentFunction))